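; Character Blueprint for a Simon Says game that switches a sprite's flipbook between idle, running and action animations.
; Pressing PerformAction plays the DoCycle animation, then after a two-second delay picks running or idle based on whether the movement component is moving.
; Tick runs that same movement check whenever the current flipbook differs from a compared flipbook, bypassing the delay.
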(event EventBeginPlay)

(event EventActorBeginOverlap
  (params (OtherActor :type Actor%20Object%20Reference)))

(event EventTick
  (params (DeltaSeconds :type Float%20%28single-precision%29))
  (if (not (== (Variables|Default|GetFlipbook) (Class|PaperFlipbookComponent|GetFlipbook (Variables|Default|Getm_sprite))))
    (if (Class|MainCharacterMovementComponent|GetIsMoving (Variables|Default|Getm_movementComponent))
      (Sprite|SetFlipbook (Variables|Default|Getm_sprite) "/Game/2dSideScroller/Sprites/RunningAnimation.RunningAnimation")
      (else
        (Sprite|SetFlipbook (Variables|Default|Getm_sprite) "/Game/2dSideScroller/Sprites/IdleAnimation.IdleAnimation")))))

(event Input|ActionEvents|InputActionPerformAction
  (params (Key :type Key%20Structure :default "AnyKey"))
  (:Pressed
    (Sprite|SetFlipbook (Variables|Default|Getm_sprite) "/Game/2DSideScroller/Sprites/DoCycleAnimation.DoCycleAnimation")
    (Utilities|FlowControl|Delay 2.0)
    (if (Class|MainCharacterMovementComponent|GetIsMoving (Variables|Default|Getm_movementComponent))
      (Sprite|SetFlipbook (Variables|Default|Getm_sprite) "/Game/2dSideScroller/Sprites/RunningAnimation.RunningAnimation")
      (else
        (Sprite|SetFlipbook (Variables|Default|Getm_sprite) "/Game/2dSideScroller/Sprites/IdleAnimation.IdleAnimation")))))

(fn ConstructionScript)