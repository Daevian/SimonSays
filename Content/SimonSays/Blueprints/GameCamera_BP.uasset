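; GameCamera_BP is an orthographic game camera that stays centred on the room the player character currently occupies.
; Every Tick it snaps to the X and Z of the MainCharacter's current room while keeping its own Y.
; BeginPlay enables player input and caches all room actors, though the graph never reads that list.
; The ZoomIn axis adds its value to OrthoWidth to zoom, with no clamping.
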(event EventBeginPlay
  (bind _outactors (Actor|GetAllActorsOfClass (Variables|Default|GetromClassREf)))
  (Variables|Default|Setrooms _outactors)
  (Input|EnableInput (Game|GetPlayerController 0)))

(event EventTick
  (params (DeltaSeconds :type Float%20%28single-precision%29))
  (bind _returnvalue (Game|Player|GetPlayerPawn 0))
  (bind _self self)
  (bind _asmain_character (Utilities|Casting|CastToMainCharacter _returnvalue))
  (bind _returnvalue_2 (Class|MainCharacter|GetCurrentRoom _asmain_character))
  (bind _returnvalue_3 (Transformation|GetActorLocation _returnvalue_2))
  (bind _output_get (Variables|Default|Settemp (Math|Vector|MakeVector (.x _returnvalue_3) (.y (Transformation|GetActorLocation _self)) (.z _returnvalue_3))))
  (Transformation|SetActorLocation _self _output_get false false))

(event Input|AxisEvents|InputAxisZoomIn
  (params (AxisValue :type Float%20%28single-precision%29))
  (bind _cameracomponent (Variables|Default|GetCameraComponent))
  ;[1 0.2397 0.9321] Camera Zoom
  (Variables|/Script/Engine.CameraComponent|SetOrthoWidth _cameracomponent (+ AxisValue (Variables|/Script/Engine.CameraComponent|GetOrthoWidth _cameracomponent))))

(fn ConstructionScript)